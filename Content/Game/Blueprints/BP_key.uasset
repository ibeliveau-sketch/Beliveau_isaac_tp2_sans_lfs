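; BP_key is a collectible key pickup that completes a secondary quest in level 2.
; The first overlap with its Box, guarded by a DoOnce, plays a sound, sets HasKey and prints a pickup message.
; It then casts the player's HUD to BP_HUD_Niveau2, sets the quest flag, refreshes the quest widget through UptdateQuest2 and hides the mesh without destroying the actor.
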(event OnComponentBeginOverlap(Box)
  (params (OverlappedComponent :type Primitive%20Component%20Object%20Reference) (OtherActor :type Actor%20Object%20Reference) (OtherComp :type Primitive%20Component%20Object%20Reference) (OtherBodyIndex :type Integer) (bFromSweep :type Boolean) (SweepResult :type Hit%20Result%20Structure%20%28by%20ref%29))
  (Utilities|FlowControl|DoOnce false
    (:Completed
      (Audio|PlaySound2D "/Game/Sound/A_collectcoin-6075.A_collectcoin-6075" 1.0 1.0 0.0 0 0)
      (Variables|Default|SetHas%20Key true)
      (Development|PrintString "Clé obtenue!")
      (bind _asbp_hud_niveau_2 (Utilities|Casting|CastToBP_HUD_Niveau2 (HUD|GetHUD (Game|GetPlayerController 0))))
      (bind _output_get (Variables|Default|SetAs%20BP%20HUD%20Niveau%202 _asbp_hud_niveau_2))
      (Variables|/Game/Game/Blueprints/BP_HUD_Niveau2.BP_HUD_Niveau2_C|SetNiv2%20Quête%20Second%202%20Complèté _output_get true)
      (Default|UptdateQuest2 (Variables|/Game/Game/Blueprints/BP_HUD_Niveau2.BP_HUD_Niveau2_C|GetReference%20Widget _output_get))
      (Rendering|SetVisibility (Variables|Debug|GetStaticMeshComponent) false false))))

(fn ConstructionScript)