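; BP_Clé is a key pickup for level 1, collected through its Obtentiondelaclé event.
; The event slides the key mesh to a fixed relative position and rotation over a few seconds, with a DoOnce guarding the follow-up.
; That follow-up plays a coin sound, prints a message, sets HasKey, then casts to BP_HUD_Niveau1 to complete the secondary objective and change its widget icon.
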(event Custom|Obtention%20de%20la%20clé
  (Components|MoveComponentTo (Variables|Debug|GetStaticMeshComponent) "-2344.867571,349.344307,528.371811" "0.000000,0.000000,-90.086323" false false 3.0 false)
  (Utilities|FlowControl|DoOnce false
    (:Completed
      (Audio|PlaySound2D "/Game/Sound/collectcoin-6075.collectcoin-6075" 1.0 1.0 0.0 0 0)
      (Development|PrintString "Clé obtenue!")
      (Variables|Default|Sethas%20key true)
      (bind _asbp_hud_niveau_1 (Utilities|Casting|CastToBP_HUD_Niveau1 (HUD|GetHUD (Game|GetPlayerController 0))))
      (Variables|/Game/Game/Blueprints/WBP_QuêteSecondaire.WBP_QuêteSecondaire_C|SetObjectifSecondaireCompleté (Variables|/Game/Game/Blueprints/BP_HUD_Niveau1.BP_HUD_Niveau1_C|GetReferenceWidget _asbp_hud_niveau_1) true)
      (Default|ChangerIcone (Variables|/Game/Game/Blueprints/BP_HUD_Niveau1.BP_HUD_Niveau1_C|GetReferenceWidget _asbp_hud_niveau_1)))))

(fn ConstructionScript)