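; BP_Porte is a door actor that opens on demand and completes the main quest objective of level 1.
; Its OuvrirPorte event plays audio, slides and rotates the door mesh over four seconds with MoveComponentTo, and sets an open flag.
; It then gets the level 1 HUD through a cast and marks the main quest widget objective complete, updating its icon.
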(event Custom|OuvrirPorte
  ;[0.15 0.15 0.15 0.5] Mouvement de la porte
  (Audio|Components|Audio|Play (Variables|Default|GetAudio) 4.0)
  (Components|MoveComponentTo (Variables|Debug|GetStaticMeshComponent) "-58.193419,-213.291711,471.000017" "0.000000,-90.000000,0.000000" false false 4.0 false)
  (Variables|Default|Setopen%20door true)
  (bind _asbp_hud_niveau_1 (Utilities|Casting|CastToBP_HUD_Niveau1 (HUD|GetHUD (Game|GetPlayerController 0))))
  (Variables|/Game/Game/Blueprints/WBP_QuêtePrincipale.WBP_QuêtePrincipale_C|SetObjectifPrincipalComplèté (Variables|/Game/Game/Blueprints/BP_HUD_Niveau1.BP_HUD_Niveau1_C|GetWidget%20Quete%20Principale _asbp_hud_niveau_1) true)
  (Default|ChangerIcone2 (Variables|/Game/Game/Blueprints/BP_HUD_Niveau1.BP_HUD_Niveau1_C|GetWidget%20Quete%20Principale _asbp_hud_niveau_1)))

(fn ConstructionScript)