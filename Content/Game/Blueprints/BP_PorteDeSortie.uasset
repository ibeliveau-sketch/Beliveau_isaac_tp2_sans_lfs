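; BP_PorteDeSortie is the Level 2 exit door, which opens on the OuvrirSortie event if a box overlap has flagged it as openable.
; The box also shows and hides an instruction prompt.
; Opening plays audio, slides the mesh to a hardcoded transform with MoveComponentTo, then marks the main objective complete and shows the level end through BP_HUD_Niveau2.
; OuvrirSortie has no caller here, and overlaps do not filter the actor.
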(event OnComponentBeginOverlap(Box)
  (params (OverlappedComponent :type Primitive%20Component%20Object%20Reference) (OtherActor :type Actor%20Object%20Reference) (OtherComp :type Primitive%20Component%20Object%20Reference) (OtherBodyIndex :type Integer) (bFromSweep :type Boolean) (SweepResult :type Hit%20Result%20Structure%20%28by%20ref%29))
  (Variables|Default|SetOuvrable true)
  (if (not (Variables|Default|GetPlayer%20Enter%20Zone))
    (Rendering|SetVisibility (Variables|Default|GetInstruction) true false)))

(event OnComponentEndOverlap(Box)
  (params (OverlappedComponent :type Primitive%20Component%20Object%20Reference) (OtherActor :type Actor%20Object%20Reference) (OtherComp :type Primitive%20Component%20Object%20Reference) (OtherBodyIndex :type Integer))
  (Variables|Default|SetOuvrable false)
  (Rendering|SetVisibility (Variables|Default|GetInstruction) false false))

(event Custom|Ouvrir%20Sortie
  (Rendering|SetVisibility (Variables|Default|GetInstruction) false false)
  (if (Variables|Default|GetOuvrable)
    (Audio|Components|Audio|Play (Variables|Default|GetAudio) 0.0)
    (Components|MoveComponentTo (Variables|Debug|GetStaticMeshComponent) "179.579372,2347.029932,106.460623" "0.000000,92.224945,0.000000" false false 5.0 false)
    (Variables|Default|SetOpen%20Door true)
    (bind _asbp_hud_niveau_2 (Utilities|Casting|CastToBP_HUD_Niveau2 (HUD|GetHUD (Game|GetPlayerController 0))))
    (Variables|/Game/Game/Widget/WBP_Quête_Principale_Niveau2.WBP_Quête_Principale_Niveau2_C|SetObjectif%20Principale%20Niv2%20Complèté (Variables|Default|GetCible) true)
    (Default|MontrerFinNiveau2 (Variables|Default|GetTarget))))

(fn ConstructionScript)