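; HUD Blueprint for level 2 that displays the quest and end-of-level widgets.
; BeginPlay creates the first secondary quest widget and adds it to the viewport.
; Custom events do the same for the second secondary quest, the main quest and the end-of-level screen when called.
; Each widget is stored in its own reference variable, and none is removed or hidden here.
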(event Custom|Montrer2èmeQuêteSecondaire
  (bind _returnvalue (UserInterface|CreateWidget "/Game/Game/Blueprints/WBP_Quête_Secondaire2_Nv2.WBP_Quête_Secondaire2_Nv2_C" (Game|GetPlayerController 0)))
  (bind _output_get (Variables|Default|SetReference%20Widget2 _returnvalue))
  (UserInterface|Viewport|AddtoViewport _output_get 0))

(event Custom|Montrer%20quête%20principale
  (bind _returnvalue (UserInterface|CreateWidget "/Game/Game/Blueprints/WBP_QuêtePrincipale.WBP_QuêtePrincipale_C" (Game|GetPlayerController 0)))
  (bind _output_get (Variables|Default|SetReference%20Widget%203 _returnvalue))
  (UserInterface|Viewport|AddtoViewport _output_get 0))

(event Custom|Fin%20Du%20Niveau2
  (bind _returnvalue (UserInterface|CreateWidget "/Game/Game/Blueprints/WBP_FinNv2.WBP_FinNv2_C" (Game|GetPlayerController 0)))
  (bind _output_get (Variables|Default|SetReference%20Widget%204 _returnvalue))
  (UserInterface|Viewport|AddtoViewport _output_get 0))

(event EventBeginPlay
  (bind _returnvalue (UserInterface|CreateWidget "/Game/Game/Blueprints/WBP_Quête_Secondaire1_Niveau2.WBP_Quête_Secondaire1_Niveau2_C" (Game|GetPlayerController 0)))
  (bind _output_get (Variables|Default|SetReference%20Widget _returnvalue))
  (UserInterface|Viewport|AddtoViewport _output_get 0))

(fn ConstructionScript)